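; BP_robotito is a robot Blueprint that carries a name, current health, maximum health and damage as variables.
; On BeginPlay it prints them as two on-screen debug messages built with Append, the second in orange with a duration set by a variable.
; Tick and the construction script do nothing, and a leftover tick debug print is disconnected.
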(event EventBeginPlay
  (Development|PrintString (Utilities|String|Append "Nombre: 
" (Variables|Default|GetNombre) " 
Vida Actual: 
" (Utilities|String|ToString(Float) (Variables|Default|GetVida))) true true "(R=0.000000,G=0.660000,B=1.000000,A=1.000000)" 15.0)
  (Development|PrintString (Utilities|String|Append "Vida Maxima: 
" (Utilities|String|ToString(Float) (Variables|Default|GetVidamaxima)) " 
Tiene de Daño: 
" (Utilities|String|ToString(Float) (Variables|Default|GetDaño))) true true "(R=1.000000,G=0.471167,B=0.058977,A=1.000000)" (Variables|Default|GetTiempodeMensaje)))

(event EventTick
  (params (DeltaSeconds :type Float%20%28single-precision%29)))

(fn ConstructionScript)
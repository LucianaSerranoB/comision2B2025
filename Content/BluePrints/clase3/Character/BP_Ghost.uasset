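; BP_Ghost is a player-controlled flipbook character that moves along the world X axis, jumps and crouches.
; BeginPlay adds its Enhanced Input mapping context, and input actions drive those movements.
; Overlaps send an InteractuableMessage to the other actor, while events for stars and damage update a running total and clamped health.
; Results, including death, are only printed on screen; flipbook switching is left unconnected.
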(event Input|EnhancedActionEvents|EnhancedInputActionIA_Movimiento
  (params (ActionValue :type Float%20%28double-precision%29) (ElapsedSeconds :type Float%20%28double-precision%29) (TriggeredSeconds :type Float%20%28double-precision%29) (InputAction :type Input%20Action%20Object%20Reference :default "/Game/BluePrints/clase3/Character/Input/Action/IA_Movimiento.IA_Movimiento"))
  (Pawn|Input|AddMovementInput "1.000000,0.000000,0.000000" ActionValue false))

(event Input|EnhancedActionEvents|EnhancedInputActionIA_Saltar
  (params (ActionValue :type Boolean) (ElapsedSeconds :type Float%20%28double-precision%29) (TriggeredSeconds :type Float%20%28double-precision%29) (InputAction :type Input%20Action%20Object%20Reference :default "/Game/BluePrints/clase3/Character/Input/Action/IA_Saltar.IA_Saltar"))
  (:Started
    (Character|Jump))
  (:Completed
    (Character|StopJumping)))

(event Input|EnhancedActionEvents|EnhancedInputActionIA_Agacharse
  (params (ActionValue :type Boolean) (ElapsedSeconds :type Float%20%28double-precision%29) (TriggeredSeconds :type Float%20%28double-precision%29) (InputAction :type Input%20Action%20Object%20Reference :default "/Game/BluePrints/clase3/Character/Input/Action/IA_Agacharse.IA_Agacharse"))
  (:Started
    (Character|Crouch))
  (:Completed
    (Character|UnCrouch)))

(event EventBeginPlay
  (bind _asplayer_controller (Utilities|Casting|CastToPlayerController (Pawn|GetController)))
  (Input|AddMappingContext (PlayerController|LocalPlayerSubsystems|GetEnhancedInputLocalPlayerSubsystem _asplayer_controller) "/Game/BluePrints/clase3/Character/Input/IMC_GhostMaping.IMC_GhostMaping" 0 "(bIgnoreAllPressedKeysUntilRelease=True,bForceImmediately=False,bNotifyUserSettings=False)"))

(event Collision|EventActorBeginOverlap
  (params (OtherActor :type Actor%20Object%20Reference))
  (Class|BPIInteractuable|Interactuable(Message) OtherActor))

(event EventDañoARealizar
  (params (Daño :type Float%20%28double-precision%29))
  (CallFunction|DañoARecibir Daño))

(event EventAgregarEstrellas
  (params (Estrellas :type Integer))
  (CallFunction|SumarEstrellas Estrellas))

(fn ConstructionScript)

(fn SumarEstrellas
  (params (Estrellas%20Entrantes :type Integer))
  (bind _output_get (Variables|Default|SetEstrella (+ Estrellas%20Entrantes (Variables|Default|GetEstrella))))
  (Development|PrintString (Utilities|String|Append "Tus Estrellas son:" (Utilities|String|ToString(Integer) _output_get))))

(fn DañoARecibir
  (params (Daño :type Float%20%28double-precision%29))
  (bind _output_get (Variables|Default|SetVidaActual (Math|Float|Clamp(Float) (- (Variables|Default|GetVidaActual) Daño) 0.0 1e+02)))
  (if (> (Variables|Default|GetVidaActual) 0.0)
    (Development|PrintString (Utilities|String|Append "Recibiste Daño:" (Utilities|String|ToString(Float) Daño) " 
Tu Vida Actual es: 
" (Utilities|String|ToString(Float) _output_get)) true true "(R=1.000000,G=0.000000,B=0.028356,A=1.000000)")
    (else
      (Development|PrintString "Moriste:" true true "(R=0.896977,G=0.000000,B=1.000000,A=1.000000)"))))